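; BunnyKillable is a Blueprint, built around its owning actor, that handles killing a bunny.
; Its OnKill event proceeds only if the player character is a PlayerBlueprint with CanKill set.
; It then plays a pop sound and spawns a blood particle effect at the owner's location.
; Finally it increments the bunny kill count in the GameData game instance and destroys the owner, which requires that cast to succeed.
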(event EventBeginPlay)

(event EventTick
  (params (DeltaSeconds :type Float%20%28single-precision%29)))

(event EventOnKill
  (bind _returnvalue (Components|GetOwner))
  (bind _asplayer_blueprint (Utilities|Casting|CastToPlayerBlueprint (Game|GetPlayerCharacter 0)))
  (if (Variables|/Game/Blueprints/PlayerBlueprint.PlayerBlueprint_C|GetCanKill _asplayer_blueprint)
    (Audio|PlaySound2D "/Game/Audio/BunnaPop.BunnaPop" 0.1)
    (Effects|SpawnEmitteratLocation "/Game/Particles/prt_bunnyblood.prt_bunnyblood" (Transformation|GetActorLocation _returnvalue))
    (bind _asgame_data (Utilities|Casting|CastToGameData (Game|GetGameInstance)))
    (Math|Integer|IncrementInt (Variables|/Game/Blueprints/GameData.GameData_C|GetNumBunniesKilled _asgame_data)
      (:%20%20
        (Actor|DestroyActor _returnvalue)))))