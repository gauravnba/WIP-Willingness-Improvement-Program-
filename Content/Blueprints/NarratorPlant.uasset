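; NarratorPlant is a trigger actor with a spinning coin mesh that plays the player's escape narration and sends them to the WhiteRoom level.
; On player overlap it sets HasEscaped on the GameData instance, freezes the player and plays a narrator line.
; Tick rotates the coin each frame and, once the player's CanMove is true again, clears SoundPlayed, fades the camera to white and loads the level.
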(event EventBeginPlay)

(event Collision|EventActorBeginOverlap
  (params (OtherActor :type Actor%20Object%20Reference))
  (bind _asplayer_character (Utilities|Casting|CastToPlayerCharacter (Game|Player|GetPlayerPawn 0)))
  (if (== OtherActor _asplayer_character)
    (if (not (Variables|Default|GetSoundPlayed))
      (bind _asgame_data (Utilities|Casting|CastToGameData (Game|GetGameInstance)))
      (Variables|/Game/Blueprints/GameData.GameData_C|SetHasEscaped _asgame_data true)
      (bind _asplayer_character_2 (Utilities|Casting|CastToPlayerCharacter (Game|Player|GetPlayerPawn 0)))
      (Class|PlayerCharacter|Freeze _asplayer_character_2)
      (Audio|PlaySound2D "/Game/Audio/Narrator014.Narrator014")
      (Variables|Default|SetSoundPlayed true))))

(event EventTick
  (params (DeltaSeconds :type Float%20%28single-precision%29))
  (bind _fadelength (Variables|Default|GetFadeLength))
  (Transformation|AddLocalRotation (Variables|Default|GetCoin_FBX) "0.000000,1.000000,0.000000" false false)
  (if (Variables|Default|GetSoundPlayed)
    (bind _asplayer_character (Utilities|Casting|CastToPlayerCharacter (Game|Player|GetPlayerPawn 0)))
    (if (Variables|/Script/WIP.PlayerCharacter|GetbCanMove _asplayer_character)
      (Variables|Default|SetSoundPlayed false)
      (CameraFades|StartCameraFade (Game|GetPlayerCameraManager 0) 0.0 1.0 _fadelength "(R=1.000000,G=1.000000,B=1.000000,A=1.000000)" false true)
      (Utilities|FlowControl|Delay _fadelength)
      (Game|OpenLevel(byName) "WhiteRoom"))))

(fn ConstructionScript)