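; Test tree actor that manually swaps between a high-detail and a low-poly version of the same tree.
; SwitchTreeLOD flips the ToggleLOD boolean and sets Hidden In Game on the HighTreeFBX and TreeLowPoly components so one shows while the other hides.
; The event graph and construction script are empty, so nothing in this Blueprint calls the switch.
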(event EventBeginPlay)

(event Collision|EventActorBeginOverlap
  (params (OtherActor :type Actor%20Object%20Reference)))

(event EventTick
  (params (DeltaSeconds :type Float%20%28single-precision%29)))

(fn ConstructionScript)

(fn SwitchTreeLOD
  (if (Variables|Default|GettoggleLOD)
    (Development|SetHiddeninGame (Variables|Default|GetHigh_Tree_FBX) true false)
    (Development|SetHiddeninGame (Variables|Default|Gettree_lowPoly) false false)
    (Variables|Default|SettoggleLOD false)
    (else
      (Development|SetHiddeninGame (Variables|Default|GetHigh_Tree_FBX) false false)
      (Development|SetHiddeninGame (Variables|Default|Gettree_lowPoly) true false)
      (Variables|Default|SettoggleLOD true))))