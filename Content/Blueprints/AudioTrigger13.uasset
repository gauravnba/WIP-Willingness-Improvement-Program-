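; AudioTrigger13 is an overlap trigger that plays two narrator lines when the player character enters it.
; On begin overlap it confirms the actor is the player pawn, plays the first 2D sound, then the second after a fixed delay.
; The SoundPlaying flag blocks replays and is never reset; it is set after the second line, or when any actor ends overlap, even one other than the player.
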(event EventBeginPlay)

(event Collision|EventActorBeginOverlap
  (params (OtherActor :type Actor%20Object%20Reference))
  (bind _asplayer_character (Utilities|Casting|CastToPlayerCharacter (Game|Player|GetPlayerPawn 0)))
  (if (== OtherActor _asplayer_character)
    (if (not (Variables|Default|GetSoundPlaying))
      (Audio|PlaySound2D "/Game/Audio/Narration/NewNarrator017.NewNarrator017")
      (Utilities|FlowControl|Delay 7.0)
      (Audio|PlaySound2D "/Game/Audio/Narration/NewNarrator018.NewNarrator018")
      (Variables|Default|SetSoundPlaying true))))

(event EventTick
  (params (DeltaSeconds :type Float%20%28single-precision%29)))

(event Collision|EventActorEndOverlap
  (params (OtherActor :type Actor%20Object%20Reference))
  (Variables|Default|SetSoundPlaying true))

(fn ConstructionScript)