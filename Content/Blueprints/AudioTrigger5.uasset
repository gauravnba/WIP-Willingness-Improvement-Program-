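; AudioTrigger5 is a trigger actor that plays a narrator voice line when the player walks into it.
; On actor overlap it confirms the other actor is the PlayerCharacter pawn, then plays NewNarrator006 as 2D sound.
; The SoundPlaying flag is set and never reset here, so the line plays only once.
; A disconnected branch that checks HasKilledBunny before playing a different narrator line never runs.
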(event EventBeginPlay)

(event Collision|EventActorBeginOverlap
  (params (OtherActor :type Actor%20Object%20Reference))
  (bind _asplayer_character (Utilities|Casting|CastToPlayerCharacter (Game|Player|GetPlayerPawn 0)))
  ;[1 1 1] Boolean for checking if player has killed bunny
  (if (== OtherActor _asplayer_character)
    (if (not (Variables|Default|GetSoundPlaying))
      (Audio|PlaySound2D "/Game/Audio/Narration/NewNarrator006.NewNarrator006")
      (Variables|Default|SetSoundPlaying true))))

(event EventTick
  (params (DeltaSeconds :type Float%20%28single-precision%29)))

(fn ConstructionScript)