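; ForestTrigger is a box trigger that switches the level of detail of the forest, bunnies and landscape when the player enters it.
; BeginPlay caches every tree and bunny actor.
; Player overlap switches each bunny's LOD, lowers or raises landscape detail through a material parameter collection scalar, and arms a flag.
; While armed, Tick repeatedly calls the trees' LOD switch on short delays for a few counted passes, creating a flicker.
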(event OnComponentBeginOverlap(Box)
  (params (OverlappedComponent :type Primitive%20Component%20Object%20Reference) (OtherActor :type Actor%20Object%20Reference) (OtherComp :type Primitive%20Component%20Object%20Reference) (OtherBodyIndex :type Integer) (bFromSweep :type Boolean) (SweepResult :type Hit%20Result%20Structure%20%28by%20ref%29))
  (Utilities|Casting|CastToPlayerCharacter OtherActor)
  (for _array_element (Variables|Default|GetBunnies)
    (Default|SwitchBunnyLOD _array_element)
    (CallFunction|LandscapeLODChange)
    (Variables|Default|SetswitchLOD true)))

(event EventBeginPlay
  (bind _outactors (Actor|GetAllActorsOfClass "/Game/Blueprints/Tree_LOD_Test_Blueprint.Tree_LOD_Test_Blueprint_C"))
  (Variables|Default|SetForest _outactors)
  (bind _outactors_2 (Actor|GetAllActorsOfClass "/Game/Blueprints/BunnyBlueprint.BunnyBlueprint_C"))
  (Variables|Default|SetBunnies _outactors_2))

(event EventTick
  (params (DeltaSeconds :type Float%20%28single-precision%29))
  (if (Variables|Default|GetswitchLOD)
    (if (< (Variables|Default|GetflickerTimes) 5)
      (Utilities|FlowControl|Delay 0.1)
      (Math|Integer|IncrementInt (Variables|Default|GetflickerTimes)
        (:%20%20
          (for _array_element (Variables|Default|GetForest)
            (Default|SwitchTreeLOD _array_element))))
      (else
        (Variables|Default|SetswitchLOD false)))))

(fn ConstructionScript)

(fn LandscapeLODChange
  (Rendering|Material|SetScalarParameterValue "/Game/ExampleContent/MatParamCollection.MatParamCollection" "LODScaler" 0.8 :!class /Script/Engine.KismetMaterialLibrary))