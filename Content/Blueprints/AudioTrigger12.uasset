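; AudioTrigger12 is a narration trigger actor for the trapped section, meant to play voice lines when the player sits too long.
; On player overlap with SoundPlaying true, it plays NewNarrator015, waits, then plays NewNarrator016 only if the flag is false by then.
; Escape sets the flag true as a self-described hacky cutoff, but nothing here clears it or stops playing audio.
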(event EventBeginPlay)

(event Collision|EventActorBeginOverlap
  (params (OtherActor :type Actor%20Object%20Reference))
  (bind _asplayer_character (Utilities|Casting|CastToPlayerCharacter (Game|Player|GetPlayerPawn 0)))
  (if (== OtherActor _asplayer_character)
    (if (Variables|Default|GetSoundPlaying)
      (Audio|PlaySound2D "/Game/Audio/Narration/NewNarrator015.NewNarrator015")
      (Utilities|FlowControl|Delay 5.0)
      ;[1 1 1] During trapped part for when player sits too long
      (if (not (Variables|Default|GetSoundPlaying))
        (Audio|PlaySound2D "/Game/Audio/Narration/NewNarrator016.NewNarrator016")
        (Variables|Default|SetSoundPlaying true)))))

(event EventTick
  (params (DeltaSeconds :type Float%20%28single-precision%29)))

(event Input|KeyboardEvents|Escape
  (params (Key :type Key%20Structure :default "AnyKey"))
  ;[1 1 1] Hacky Way of cutting off sound if steeping out of Trigger
  (:Pressed
    (Variables|Default|SetSoundPlaying true)))

(fn ConstructionScript)