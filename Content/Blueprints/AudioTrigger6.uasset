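; AudioTrigger6 is an overlap trigger that plays an end-of-level narrator line and completes the game.
; When the player pawn enters, PlayerCharacter's WeaponEquipped flag picks one of two narrator sounds, with SoundPlaying blocking repeats.
; Both branches then share one delayed sequence: confetti spawns at a hard-coded location, GameData's NumGamesWon increments on the game instance, and LevelTest opens.
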(event EventBeginPlay)

(event Collision|EventActorBeginOverlap
  (params (OtherActor :type Actor%20Object%20Reference))
  ;[1 1 1] Boolean for checking if player has sword
  (bind _asplayer_character (Utilities|Casting|CastToPlayerCharacter (Game|Player|GetPlayerPawn 0)))
  (if (== OtherActor _asplayer_character)
    (if (Variables|/Script/WIP.PlayerCharacter|GetbWeaponEquipped _asplayer_character)
      (if (not (Variables|Default|GetSoundPlaying))
        (Audio|PlaySound2D "/Game/Audio/Narration/NewNarrator007.NewNarrator007")
        (Variables|Default|SetSoundPlaying true :!label _label)
        (Utilities|FlowControl|Delay 12.0)
        (Effects|SpawnEmitteratLocation "/Game/Particles/prt_confetti.prt_confetti" "8961.000000,23167.000000,644.000000" "0, 0, 0" false)
        (Utilities|FlowControl|Delay 3.0)
        (bind _asgame_data (Utilities|Casting|CastToGameData (Game|GetGameInstance)))
        (Math|Integer|IncrementInt (Variables|/Game/Blueprints/GameData.GameData_C|GetNumGamesWon _asgame_data)
          (:%20%20
            (Game|OpenLevel(byName) "LevelTest"))))
      (elif (not (Variables|Default|GetSoundPlaying))
        (Audio|PlaySound2D "/Game/Audio/Narration/NewNarrator008.NewNarrator008")
        (goto _label)))))

(event EventTick
  (params (DeltaSeconds :type Float%20%28single-precision%29)))

(fn ConstructionScript)