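; AudioTrigger10 is a trigger actor that plays a 2D narrator voice line when the player character enters it.
; After a short delay on overlap, it plays the sound only if the SoundPlaying flag is unset, then sets the flag.
; Any end overlap also sets the flag, so leaving during the delay suppresses the line; the flag never resets, so the line plays at most once.
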(event EventBeginPlay)

(event Collision|EventActorBeginOverlap
  (params (OtherActor :type Actor%20Object%20Reference))
  (bind _asplayer_character (Utilities|Casting|CastToPlayerCharacter (Game|Player|GetPlayerPawn 0)))
  (if (== OtherActor _asplayer_character)
    (Utilities|FlowControl|Delay 2.0)
    (if (not (Variables|Default|GetSoundPlaying))
      (Audio|PlaySound2D "/Game/Audio/Narration/NewNarrator013.NewNarrator013")
      (Variables|Default|SetSoundPlaying true))))

(event EventTick
  (params (DeltaSeconds :type Float%20%28single-precision%29)))

(event Collision|EventActorEndOverlap
  (params (OtherActor :type Actor%20Object%20Reference))
  ;[1 1 1] Hacky Way of cutting off sound if steeping out of Trigger
  (Variables|Default|SetSoundPlaying true))

(fn ConstructionScript)