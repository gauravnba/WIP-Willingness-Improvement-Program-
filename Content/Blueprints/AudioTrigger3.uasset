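; AudioTrigger3 is a trigger actor that plays a narrator line when the player walks into it.
; On overlap it confirms the actor is the player character, then plays one of two 2D narrator sounds depending on whether a weapon is equipped.
; A SoundPlaying flag is set afterward and never cleared here, so only one line plays once per trigger.
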(event EventBeginPlay)

(event Collision|EventActorBeginOverlap
  (params (OtherActor :type Actor%20Object%20Reference))
  (bind _asplayer_character (Utilities|Casting|CastToPlayerCharacter (Game|Player|GetPlayerPawn 0)))
  (if (== OtherActor _asplayer_character)
    (if (Variables|/Script/WIP.PlayerCharacter|GetbWeaponEquipped _asplayer_character)
      (if (not (Variables|Default|GetSoundPlaying))
        (Audio|PlaySound2D "/Game/Audio/Narration/NewNarrator003.NewNarrator003")
        (Variables|Default|SetSoundPlaying true :!label _label))
      (elif (not (Variables|Default|GetSoundPlaying))
        (Audio|PlaySound2D "/Game/Audio/Narration/NewNarrator004.NewNarrator004")
        (goto _label)))))

(event EventTick
  (params (DeltaSeconds :type Float%20%28single-precision%29)))

(fn ConstructionScript)