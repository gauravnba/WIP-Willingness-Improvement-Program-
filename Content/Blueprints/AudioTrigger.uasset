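; AudioTrigger is a trigger actor that plays a narrator voice line when the player character overlaps it.
; On overlap it checks that the other actor is the player pawn and that the SoundPlaying flag is not yet set, so the line plays only once.
; It reads HasEscaped from the GameData game instance to pick an alternate line for a restart after capture.
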(event EventBeginPlay)

(event Collision|EventActorBeginOverlap
  (params (OtherActor :type Actor%20Object%20Reference))
  (bind _asplayer_character (Utilities|Casting|CastToPlayerCharacter (Game|Player|GetPlayerPawn 0)))
  (if (== OtherActor _asplayer_character)
    (if (not (Variables|Default|GetSoundPlaying))
      (bind _asgame_data (Utilities|Casting|CastToGameData (Game|GetGameInstance)))
      ;[1 1 1] If player restarts after capture
      (if (Variables|/Game/Blueprints/GameData.GameData_C|GetHasEscaped _asgame_data)
        (Audio|PlaySound2D "/Game/Audio/Narration/NewNarrator019.NewNarrator019")
        (else
          (Audio|PlaySound2D "/Game/Audio/Narration/NewNarrator001.NewNarrator001")))
      (Variables|Default|SetSoundPlaying true))))

(event EventTick
  (params (DeltaSeconds :type Float%20%28single-precision%29)))

(fn ConstructionScript)